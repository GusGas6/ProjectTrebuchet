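; Mission selection actor that lets a player character pick one of three missions (green, yellow or red) by walking into its boxes.
; Each box overlap checks for BP_ThirdPersonCharacter, then passes that mission's level name to the Game Instance through MissionSelectedMessage.
; It updates the text render to announce the selection, hides the chosen box and shows the other two.
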(event `self.Box1.OnComponentBeginOverlap`
  (params (OverlappedComponent :type "PrimitiveComponent Object Reference") (OtherActor :type "Actor Object Reference") (OtherComp :type "PrimitiveComponent Object Reference") (OtherBodyIndex :type Integer) (bFromSweep :type Boolean) (SweepResult :type "HitResult Structure (by ref)"))
  (if (== (`GameplayStatics.GetObjectClass` OtherActor) "/Game/Blueprints/BP_ThirdPersonCharacter.BP_ThirdPersonCharacter_C")
    (message `/Game/Blueprints/Interfaces/MissionSelect_BPI.MissionSelected` (`GameplayStatics.GetGameInstance`) "Lvl_TestActualLevel1")
    (`TextRenderComponent.K2_SetText` (`self.TextRender1`) (`KismetTextLibrary.Conv_StringToText` (`KismetStringLibrary.Concat_StrStr` "> MISSION GREEN SELECTED <")))
    (`SceneComponent.SetHiddenInGame` (`self.Box1`) true false)
    (`SceneComponent.SetHiddenInGame` (`self.Box`) false false)
    (`SceneComponent.SetHiddenInGame` (`self.Box2`) false false)))

(event `self.Box.OnComponentBeginOverlap`
  (params (OverlappedComponent :type "PrimitiveComponent Object Reference") (OtherActor :type "Actor Object Reference") (OtherComp :type "PrimitiveComponent Object Reference") (OtherBodyIndex :type Integer) (bFromSweep :type Boolean) (SweepResult :type "HitResult Structure (by ref)"))
  (if (== (`GameplayStatics.GetObjectClass` OtherActor) "/Game/Blueprints/BP_ThirdPersonCharacter.BP_ThirdPersonCharacter_C")
    (message `/Game/Blueprints/Interfaces/MissionSelect_BPI.MissionSelected` (`GameplayStatics.GetGameInstance`) "Lvl_TestActualLevel")
    (`TextRenderComponent.K2_SetText` (`self.TextRender1`) (`KismetTextLibrary.Conv_StringToText` (`KismetStringLibrary.Concat_StrStr` "> MISSION YELLOW SELECTED <")))
    (`SceneComponent.SetHiddenInGame` (`self.Box`) true false)
    (`SceneComponent.SetHiddenInGame` (`self.Box2`) false false)
    (`SceneComponent.SetHiddenInGame` (`self.Box1`) false false)))

(event `self.Box2.OnComponentBeginOverlap`
  (params (OverlappedComponent :type "PrimitiveComponent Object Reference") (OtherActor :type "Actor Object Reference") (OtherComp :type "PrimitiveComponent Object Reference") (OtherBodyIndex :type Integer) (bFromSweep :type Boolean) (SweepResult :type "HitResult Structure (by ref)"))
  (if (== (`GameplayStatics.GetObjectClass` OtherActor) "/Game/Blueprints/BP_ThirdPersonCharacter.BP_ThirdPersonCharacter_C")
    (message `/Game/Blueprints/Interfaces/MissionSelect_BPI.MissionSelected` (`GameplayStatics.GetGameInstance`) "Lvl_TestActualLevel2")
    (`TextRenderComponent.K2_SetText` (`self.TextRender1`) (`KismetTextLibrary.Conv_StringToText` (`KismetStringLibrary.Concat_StrStr` "> MISSION RED SELECTED <")))
    (`SceneComponent.SetHiddenInGame` (`self.Box2`) true false)
    (`SceneComponent.SetHiddenInGame` (`self.Box1`) false false)
    (`SceneComponent.SetHiddenInGame` (`self.Box`) false false)))

(fn `UserConstructionScript`)