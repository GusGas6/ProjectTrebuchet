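; Multiplayer hub drop pod that launches the party to the next selected level once all networked players stand inside its capsule.
; Overlap events count player characters and update the text and light, running a delay-loop countdown while everyone is present.
; At zero, authority and remote both fade the camera, then authority server-travels to the level stored in the game instance.
; The pod registers itself with that game instance; MissionSelected destroys its static mesh once.
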(event `self.ReceiveBeginPlay`
  (`KismetSystemLibrary.DelayUntilNextTick`)
  (bind _asbp_online_game_instance (cast `/Game/Blueprints/Online/BP_OnlineGameInstance` (`GameplayStatics.GetGameInstance`)))
  (set `/Game/Blueprints/Online/BP_OnlineGameInstance.DropPodREF` self _asbp_online_game_instance))

(event `self.Capsule.OnComponentBeginOverlap`
  (params (OverlappedComponent :type "PrimitiveComponent Object Reference") (OtherActor :type "Actor Object Reference") (OtherComp :type "PrimitiveComponent Object Reference") (OtherBodyIndex :type Integer) (bFromSweep :type Boolean) (SweepResult :type "HitResult Structure (by ref)"))
  (bind _numnetplayers (`AdvancedSessionsLibrary.GetNumberOfNetworkPlayers`))
  (bind _textrender (`self.TextRender`))
  (bind _timeuntillaunch (`self.TimeUntilLaunch`))
  (bind _overlappingplayers (`self.OverlappingPlayers`))
  (if (== (`GameplayStatics.GetObjectClass` OtherActor) "/Game/Blueprints/BP_ThirdPersonCharacter.BP_ThirdPersonCharacter_C")
    (`/Engine/EditorBlueprintResources/StandardMacros.IncrementInt` _overlappingplayers
      (:`  `
        (if (>= _overlappingplayers _numnetplayers) :!label _label
          (`SceneComponent.SetHiddenInGame` _textrender false false)
          (bind _output_get (set `self.TimeUntilLaunch` (- _timeuntillaunch 0.1)))
          (`LightComponent.SetLightColor` (`self.PointLight`) (struct :`G` 1.0 :`B` 0.017766 :`A` 1.0) true)
          (if (<= _output_get 0.0)
            (`/Engine/EditorBlueprintResources/ActorMacros.Switch Has Authority`
              (:`Authority`
                (`PlayerCameraManager.StartCameraFade` :`self` (`GameplayStatics.GetPlayerCameraManager` 0) :`ToAlpha` 1.0 :`Duration` 1.0 :`bHoldWhenFinished` true)
                (`KismetSystemLibrary.Delay` 2.0)
                (bind _asbp_online_game_instance (cast `/Game/Blueprints/Online/BP_OnlineGameInstance` (`GameplayStatics.GetGameInstance`)))
                (`AdvancedSessionsLibrary.ServerTravel` (`KismetStringLibrary.Conv_NameToString` (`/Game/Blueprints/Online/BP_OnlineGameInstance.NextSelectedLevel` _asbp_online_game_instance)) true))
              (:`Remote`
                (`PlayerCameraManager.StartCameraFade` :`self` (`GameplayStatics.GetPlayerCameraManager` 0) :`ToAlpha` 1.0 :`Duration` 1.0 :`bHoldWhenFinished` true)))
            (else
              (`TextRenderComponent.K2_SetText` (`self.TextRender`) (`KismetTextLibrary.Conv_StringToText` (`KismetStringLibrary.Concat_StrStr` "LAUNCHING IN... " (`KismetStringLibrary.Conv_IntToString` (+ (`KismetMathLibrary.FTrunc` _timeuntillaunch) 1)))))
              (`KismetSystemLibrary.Delay` 0.1)
              (goto _label)))
          (else
            (`TextRenderComponent.K2_SetText` _textrender (`KismetTextLibrary.Conv_StringToText` (`KismetStringLibrary.Concat_StrStr` (`KismetStringLibrary.Conv_IntToString` _overlappingplayers) " / " (`KismetStringLibrary.Conv_IntToString` _numnetplayers) " PLAYERS")))
            (set `self.TimeUntilLaunch` 5.0)
            (`SceneComponent.SetHiddenInGame` _textrender false false)
            (`LightComponent.SetLightColor` (`self.PointLight`) (struct :`R` 1.0 :`G` 0.057609 :`A` 1.0) true)))))))

(event `self.Capsule.OnComponentEndOverlap`
  (params (OverlappedComponent :type "PrimitiveComponent Object Reference") (OtherActor :type "Actor Object Reference") (OtherComp :type "PrimitiveComponent Object Reference") (OtherBodyIndex :type Integer))
  (if (== (`GameplayStatics.GetObjectClass` OtherActor) "/Game/Blueprints/BP_ThirdPersonCharacter.BP_ThirdPersonCharacter_C")
    (bind _output_get (set `self.OverlappingPlayers` (`KismetMathLibrary.Clamp` (- (`self.OverlappingPlayers`) 1) 0 999)))
    (if (<= _output_get 0)
      (`SceneComponent.SetHiddenInGame` (`self.TextRender`) true false)
      (`LightComponent.SetLightColor` (`self.PointLight`) (struct :`R` 1.0 :`G` 0.057609 :`A` 1.0) true))))

(event `/Game/Blueprints/Interfaces/CoOp_BPI.MissionSelected`
  (params (MissionName :type Text))
  (bind _staticmesh (`self.StaticMesh`))
  ;[0.15 0.02772 0.001066 0.5] TODO: Be able to close door if mission deselected
  (`/Engine/EditorBlueprintResources/StandardMacros.DoOnce` false
    (:`Completed`
      (`/Engine/EditorBlueprintResources/StandardMacros.IsValid` _staticmesh
        (:`Is Valid`
          (`ActorComponent.K2_DestroyComponent` _staticmesh))))))

(fn `UserConstructionScript`)