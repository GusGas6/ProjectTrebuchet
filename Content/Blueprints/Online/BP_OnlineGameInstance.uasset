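; Online game instance that handles session hosting, invite joins, drop pod mission selection and player sync.
; Hosting opens the third-person map as a listen server; both received and accepted invites destroy any existing session, then join through a transition map.
; Server-to-client events trigger progress sync on every player pawn.
; A one-second server loop sends player IDs to clients, which apply Steam avatars to character materials and debug-print IDs.
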(event `CreateSession`
  ; Create Session
  (bind _sessionstate (`AdvancedSessionsLibrary.GetSessionState`))
  (if (not (`|EnumEquality` _sessionstate "NoSession"))
    (`DestroySessionCallbackProxy.DestroySession` (`GameplayStatics.GetPlayerController` 0)
      (:`OnSuccess`
        (`KismetSystemLibrary.PrintString` "DESTROYING SESSION TO JOIN FRIEND" true true (struct :`R` 0.002999 :`G` 1.0 :`A` 1.0) 15.0))
      (:`OnFailure`
        (`KismetSystemLibrary.PrintString` "FAILED TO DESTROY SESSION" true true (struct :`R` 1.0 :`B` 0.163893 :`A` 1.0) 15.0))))
  (`CreateSessionCallbackProxyAdvanced.CreateAdvancedSession` :`PlayerController` (`GameplayStatics.GetPlayerController` 0)
    (:`OnSuccess`
      (`GameplayStatics.OpenLevelBySoftObjectPtr` "/Game/Levels/Lvl_ThirdPerson.Lvl_ThirdPerson" true "listen"))))

(event `self.OnSessionInviteAccepted`
  (params (LocalPlayerNum :type Integer) (PersonInvited :type "BPUniqueNetId Structure") (SessionToJoin :type "BlueprintSessionResult Structure (by ref)"))
  ; Join Session (via invite)
  (`|ExecutionSequence`
    (:`then_0`
      (bind _sessionstate (`AdvancedSessionsLibrary.GetSessionState`))
      (if (`|EnumEquality` _sessionstate "NoSession")
        (`GameplayStatics.OpenLevelBySoftObjectPtr` "/Game/UI/UI_Levels/TransitionMap.TransitionMap" :!label _label)
        (`KismetSystemLibrary.Delay` 2.0)
        (`JoinSessionCallbackProxy.JoinSession` (`GameplayStatics.GetPlayerController` 0) SessionToJoin
          (:`OnFailure`
            ;; Failure Anim Here
            (`KismetSystemLibrary.PrintString` "FAILED TO JOIN")))
        (else
          (`DestroySessionCallbackProxy.DestroySession` (`GameplayStatics.GetPlayerController` 0)
            (:`then`
              (goto _label))
            (:`OnSuccess`
              (`KismetSystemLibrary.PrintString` "DESTROYING SESSION TO JOIN FRIEND" true true (struct :`R` 0.002999 :`G` 1.0 :`A` 1.0) 15.0))
            (:`OnFailure`
              (`KismetSystemLibrary.PrintString` "FAILED TO DESTROY SESSION" true true (struct :`R` 1.0 :`B` 0.163893 :`A` 1.0) 15.0))))))
    (:`then_1`
      ;; Trying to Join Anim Here
      (`KismetSystemLibrary.PrintString` "TRYING TO JOIN..."))))

(event `self.OnSessionInviteReceived`
  (params (LocalPlayerNum :type Integer) (PersonInviting :type "BPUniqueNetId Structure") (AppId :type String) (SessionToJoin :type "BlueprintSessionResult Structure (by ref)"))
  ; Invite Recieved
  (`|ExecutionSequence`
    (:`then_0`
      (bind _sessionstate (`AdvancedSessionsLibrary.GetSessionState`))
      (if (`|EnumEquality` _sessionstate "NoSession")
        (`GameplayStatics.OpenLevelBySoftObjectPtr` "/Game/UI/UI_Levels/TransitionMap.TransitionMap" :!label _label_2)
        (`KismetSystemLibrary.Delay` 2.0)
        (`JoinSessionCallbackProxy.JoinSession` (`GameplayStatics.GetPlayerController` 0) SessionToJoin
          (:`OnFailure`
            ;; Failure Anim Here
            (`KismetSystemLibrary.PrintString` "FAILED TO JOIN")))
        (else
          (`DestroySessionCallbackProxy.DestroySession` (`GameplayStatics.GetPlayerController` 0)
            (:`then`
              (goto _label_2))
            (:`OnSuccess`
              (`KismetSystemLibrary.PrintString` "DESTROYING SESSION TO JOIN FRIEND" true true (struct :`R` 0.002999 :`G` 1.0 :`A` 1.0) 15.0))
            (:`OnFailure`
              (`KismetSystemLibrary.PrintString` "FAILED TO DESTROY SESSION" true true (struct :`R` 1.0 :`B` 0.163893 :`A` 1.0) 15.0))))))
    (:`then_1`
      ;; Trying to Join Anim Here
      (`KismetSystemLibrary.PrintString` "TRYING TO JOIN..."))))

(event `/Game/Blueprints/Interfaces/CoOp_BPI.MissionSelected`
  (params (MissionName :type Text))
  (bind _droppodref (`self.DropPodREF`))
  ; DropPod Mission Select
  (set `self.NextSelectedLevel` (`KismetStringLibrary.Conv_StringToName` (`KismetTextLibrary.Conv_TextToString` MissionName)))
  (`/Engine/EditorBlueprintResources/StandardMacros.IsValid` _droppodref
    (:`Is Valid`
      (message `/Game/Blueprints/Interfaces/CoOp_BPI.MissionSelected` _droppodref ""))))

(event `/Game/Blueprints/Interfaces/CoOp_BPI.SyncPlayerProgress`
  (params (PlayerREF :type "Actor Object Reference") (PlayerController :type "Controller Object Reference") (UniqueNetID :type "BPUniqueNetId Structure"))
  ; Sync player progress
  (`|ExecutionSequence`
    (:`then_0`
      (`self.SERVER_SyncPlayerProgress` PlayerController PlayerREF UniqueNetID))
    (:`then_1`
      (`self.SERVER_ReplicatePlayerArray`))))

(event `SERVER_SyncPlayerProgress`
  (params (PlayerController :type "Controller Object Reference (by ref)") (PlayerREF :type "Actor Object Reference (by ref)") (ItemToFind :type "BPUniqueNetId Structure (by ref)"))
  ; Sync player progress
  (`self.CLIENT_SyncPlayerProgress` PlayerController PlayerREF ItemToFind))

(event `CLIENT_SyncPlayerProgress`
  (params (PlayerController :type "Controller Object Reference (by ref)") (PlayerREF :type "Actor Object Reference (by ref)") (ItemToFind :type "BPUniqueNetId Structure (by ref)"))
  ; Sync player progress
  (for _array_element (`GameStateBase.PlayerArray` (`GameplayStatics.GetGameState`))
    (message `/Game/Blueprints/Interfaces/CoOp_BPI.SyncPlayerProgress` (`PlayerState.GetPawn` _array_element) null null (struct))))

(event `SERVER_ReplicatePlayerArray`
  ; Update Player Avatar
  (for _array_element (`GameStateBase.PlayerArray` (`GameplayStatics.GetGameState`))
    (`self.CLIENT_UsePlayerArray` (`AdvancedSessionsLibrary.UniqueNetIdToString` (`AdvancedSessionsLibrary.GetUniqueNetIDFromPlayerState` _array_element)) _array_element))
  (`KismetSystemLibrary.Delay` 1.0)
  (`self.SERVER_ReplicatePlayerArray`))

(event `CLIENT_UsePlayerArray`
  (params (UniqueNetworkID :type String) (PlayerState :type "PlayerState Object Reference"))
  (bind _returnvalue (`AdvancedSteamFriendsLibrary.CreateSteamIDFromString` UniqueNetworkID))
  (bind _unique_net_ids (`self.Unique Net Ids`))
  ; Update Player Avatar
  (`|ExecutionSequence`
    (:`then_0`
      (bind _returnvalue_2 (`AdvancedSteamFriendsLibrary.RequestSteamFriendInfo` _returnvalue))
      (if _returnvalue_2
        (if (not (`KismetArrayLibrary.Array_Contains` _unique_net_ids _returnvalue))
          (`KismetArrayLibrary.Array_Add` _unique_net_ids _returnvalue))
        (bind _returnvalue_3 (`AdvancedSteamFriendsLibrary.GetSteamFriendAvatar` _returnvalue "SteamAvatar_Large")
          (:`OnSuccess`
            (bind _asbp_third_person_character (cast `/Game/Blueprints/BP_ThirdPersonCharacter` (`PlayerState.GetPawn` PlayerState)))
            (set `/Game/Blueprints/BP_ThirdPersonCharacter.LocalSteamAvatar` _returnvalue_3 _asbp_third_person_character)
            (bind _mesh (`Character.Mesh` _asbp_third_person_character))
            (bind _returnvalue_4 (`PrimitiveComponent.CreateDynamicMaterialInstance` _mesh 1 "/Game/CustomMaterials/SteamAvatar_Mat.SteamAvatar_Mat" "None"))
            (`PrimitiveComponent.SetMaterial` _mesh 1 _returnvalue_4)
            (`MaterialInstanceDynamic.SetTextureParameterValue` _returnvalue_4 "SteamAvatarParam" _returnvalue_3)))))
    (:`then_1`
      (`/Engine/EditorBlueprintResources/StandardMacros.DoOnce` false
        (:`Completed`
          (for (_array_element _array_index) (`self.Unique Net Ids`) :!label _label_3
            (`KismetSystemLibrary.PrintString` (`KismetStringLibrary.Concat_StrStr` "PLAYER " (`KismetStringLibrary.Conv_IntToString` _array_index) " ID:" (`AdvancedSessionsLibrary.UniqueNetIdToString` _array_element)) true false (struct :`R` 0.943846 :`G` 1.0 :`B` 0.922384 :`A` 1.0) 0.0)
            (`KismetSystemLibrary.DelayUntilNextTick`)
            (goto _label_3)))))))