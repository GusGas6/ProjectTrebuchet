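; Broadsword melee weapon actor that deals point damage to actors its hitbox overlaps while activated.
; Activate and Deactivate toggle hitbox collision and visibility through SERVER-to-CLIENT event pairs, clearing the hit-actor list so each target registers once per activation.
; New overlaps pass through a similar event pair, with damage applied in the CLIENT event and credited to the parent actor and its instigator controller.
; Debug prints show hits and, every tick, the hitbox collision state.
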(event `/Game/Blueprints/Interfaces/Weapon_BPI.Activate`
  (`self.SERVER_EnableHitbox` (`self.WeaponHitbox`) true))

(event `/Game/Blueprints/Interfaces/Weapon_BPI.Deactivate`
  (`self.SERVER_EnableHitbox` (`self.WeaponHitbox`)))

(event `SERVER_EnableHitbox`
  (params (Hitbox :type "PrimitiveComponent Object Reference") (Enable :type Boolean))
  (`self.CLIENT_EnableHitbox` Enable Hitbox))

(event `CLIENT_EnableHitbox`
  (params (Enable :type Boolean) (Hitbox :type "PrimitiveComponent Object Reference"))
  (if Enable
    (`PrimitiveComponent.SetCollisionEnabled` Hitbox "QueryAndProbe")
    (`KismetArrayLibrary.Array_Clear` (`self.HitActorsArray`))
    (`SceneComponent.SetHiddenInGame` Hitbox false false)
    (else
      (`PrimitiveComponent.SetCollisionEnabled` Hitbox "NoCollision")
      (`SceneComponent.SetHiddenInGame` Hitbox true false)
      (`KismetArrayLibrary.Array_Clear` (`self.HitActorsArray`)))))

(event `self.WeaponHitbox.OnComponentBeginOverlap`
  (params (OverlappedComponent :type "PrimitiveComponent Object Reference") (OtherActor :type "Actor Object Reference") (OtherComp :type "PrimitiveComponent Object Reference") (OtherBodyIndex :type Integer) (bFromSweep :type Boolean) (SweepResult :type "HitResult Structure (by ref)"))
  (bind _returnvalue (`self.GetParentActor`))
  (bind _hitactorsarray (`self.HitActorsArray`))
  (if (not (`KismetArrayLibrary.Array_Contains` _hitactorsarray OtherActor))
    (`KismetArrayLibrary.Array_Add` _hitactorsarray OtherActor)
    (`/Engine/EditorBlueprintResources/StandardMacros.IsValid` OtherActor
      (:`Is Valid`
        (`self.SERVER_HitEvent` OtherActor (`self.Base Damage`) (`KismetMathLibrary.GetDirectionUnitVector` (`self.K2_GetActorLocation`) (`.Location` (`GameplayStatics.BreakHitResult` SweepResult))) SweepResult _returnvalue (`self.Damage Type Class`) (`self.GetInstigatorController` _returnvalue))))))

(event `SERVER_HitEvent`
  (params (DamagedActor :type "Actor Object Reference") (BaseDamage :type "Float (single-precision)") (HitFromDirection :type "Vector Structure (by ref)") (HitInfo :type "HitResult Structure (by ref)") (DamageCauser :type "Actor Object Reference") (DamageTypeClass :type "DamageType Class Reference") (EventInstigator :type "Controller Object Reference"))
  (`self.CLIENT_HitEvent` DamagedActor BaseDamage HitFromDirection HitInfo DamageCauser DamageTypeClass EventInstigator))

(event `CLIENT_HitEvent`
  (params (DamagedActor :type "Actor Object Reference") (BaseDamage :type "Float (single-precision)") (HitFromDirection :type "Vector Structure (by ref)") (HitInfo :type "HitResult Structure (by ref)") (DamageCauser :type "Actor Object Reference") (DamageTypeClass :type "DamageType Class Reference") (EventInstigator :type "Controller Object Reference"))
  (`GameplayStatics.ApplyPointDamage` DamagedActor BaseDamage HitFromDirection HitInfo EventInstigator DamageCauser DamageTypeClass)
  (`KismetSystemLibrary.PrintString` (`KismetStringLibrary.Concat_StrStr` "HIT: " (`KismetSystemLibrary.GetDisplayName` DamagedActor))))

(event `self.ReceiveTick`
  (params (DeltaSeconds :type "Float (single-precision)"))
  (`KismetSystemLibrary.PrintString` (`|GetEnumeratorNameAsString` (`PrimitiveComponent.GetCollisionEnabled` (`self.WeaponHitbox`))) true true (struct :`G` 0.66 :`B` 1.0 :`A` 1.0) 0.0))

(fn `UserConstructionScript`)