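; Debug pickup actor for the save system that passes pink and blue hat flags to the player.
; The construction script colours the cone by those flags, with pink taking priority over blue and a third material when neither is set.
; A timeline started on BeginPlay moves the cone vertically.
; Overlapping the sphere with exactly a BP_ThirdPersonCharacter calls SaveGameMessage on it with both flags.
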(event `self.ReceiveBeginPlay`
  (bind (_direction _newtrack_0) (`Timeline|Timeline` :!via `PlayFromStart`)
    (:`Update`
      (`SceneComponent.K2_SetRelativeLocation` (`self.Cone`) (`KismetMathLibrary.VLerp` (0.0 0.0 70.0) (0.0 0.0 90.0) _newtrack_0) false false))))

(event `self.Sphere.OnComponentBeginOverlap`
  (params (OverlappedComponent :type "PrimitiveComponent Object Reference") (OtherActor :type "Actor Object Reference") (OtherComp :type "PrimitiveComponent Object Reference") (OtherBodyIndex :type Integer) (bFromSweep :type Boolean) (SweepResult :type "HitResult Structure (by ref)"))
  (if (== (`GameplayStatics.GetObjectClass` OtherActor) "/Game/Blueprints/BP_ThirdPersonCharacter.BP_ThirdPersonCharacter_C")
    (message `/Game/Blueprints/Interfaces/CoOp_BPI.SaveGame` OtherActor (`self.PinkHat`) (`self.BlueHat`))))

(fn `UserConstructionScript`
  (if (`self.PinkHat`)
    (`PrimitiveComponent.SetMaterial` (`self.Cone`) 0 "/Engine/VREditor/BasicMeshes/MI_Pyramid_01.MI_Pyramid_01")
    (elif (`self.BlueHat`)
      (`PrimitiveComponent.SetMaterial` (`self.Cone`) 0 "/AnimationSharing/AnimSharingBlue.AnimSharingBlue")
      (else
        (`PrimitiveComponent.SetMaterial` (`self.Cone`) 0 "/Engine/VREditor/LaserPointer/LaserPointerMaterial_Inst.LaserPointerMaterial_Inst")))))