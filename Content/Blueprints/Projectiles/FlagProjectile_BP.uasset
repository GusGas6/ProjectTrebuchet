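; Flag projectile that displays a Steam avatar on its mesh and plants a flag on whatever it hits.
; The avatar texture is relayed through server-to-client events into a dynamic material on the flag mesh.
; A hit takes the same relay, and the client event applies point damage, spawns an EnsignFlag_BP at the mesh transform with that avatar, attaches it to the hit component and destroys the projectile.
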(event `SERVER_SetFlagImage`
  (params (SteamAvatarTexture :type "Texture Object Reference"))
  (`self.CLIENT_SetFlagImage` SteamAvatarTexture))

(event `CLIENT_SetFlagImage`
  (params (SteamAvatarTexture :type "Texture Object Reference"))
  (bind _ensignflagmesh (`self.EnsignFlagMesh`))
  (bind _returnvalue (`PrimitiveComponent.CreateDynamicMaterialInstance` _ensignflagmesh 1 "/Game/CustomMaterials/SteamAvatar_Mat.SteamAvatar_Mat" "None"))
  (`PrimitiveComponent.SetMaterial` _ensignflagmesh 1 _returnvalue)
  (`MaterialInstanceDynamic.SetTextureParameterValue` _returnvalue "SteamAvatarParam" SteamAvatarTexture)
  (set `self.Steam Avatar Texture` SteamAvatarTexture))

(event `self.ReceiveHit`
  (params (MyComp :type "PrimitiveComponent Object Reference") (Other :type "Actor Object Reference") (OtherComp :type "PrimitiveComponent Object Reference") (bSelfMoved :type Boolean) (HitLocation :type "Vector Structure") (HitNormal :type "Vector Structure") (NormalImpulse :type "Vector Structure") (Hit :type "HitResult Structure (by ref)"))
  (bind (_bblockinghit _binitialoverlap _time _distance _location _impactpoint _normal _impactnormal _physmat _hitactor _hitcomponent) (`GameplayStatics.BreakHitResult` Hit))
  (bind _ensignflagmesh (`self.EnsignFlagMesh`))
  (`self.SERVER_EventHit` (`self.Steam Avatar Texture`) (`SceneComponent.K2_GetComponentLocation` _ensignflagmesh) (`SceneComponent.K2_GetComponentRotation` _ensignflagmesh) (`SceneComponent.K2_GetComponentScale` _ensignflagmesh) _hitcomponent (`self.Damage Type Class`) (`self.GetOwner`) Hit (`KismetMathLibrary.GetDirectionUnitVector` (`self.K2_GetActorLocation`) HitLocation) (`self.Base Damage`) _hitactor))

(event `SERVER_EventHit`
  (params (SteamAvatarTexture :type "Texture Object Reference") (`Spawn Transform Location` :type "Vector Structure") (`Spawn Transform Rotation` :type "Rotator Structure") (`Spawn Transform Scale` :type "Vector Structure") (AttachToComponent :type "SceneComponent Object Reference") (DamageTypeClass :type "DamageType Class Reference") (DamageCauser :type "Actor Object Reference") (HitInfo :type "HitResult Structure (by ref)") (HitFromDirection :type "Vector Structure (by ref)") (BaseDamage :type "Float (single-precision)") (DamagedActor :type "Actor Object Reference"))
  (`self.CLIENT_EventHit` SteamAvatarTexture `Spawn Transform Location` `Spawn Transform Rotation` `Spawn Transform Scale` AttachToComponent DamageTypeClass DamageCauser HitInfo HitFromDirection BaseDamage DamagedActor))

(event `CLIENT_EventHit`
  (params (SteamAvatarTexture :type "Texture Object Reference") (`Spawn Transform Location` :type "Vector Structure") (`Spawn Transform Rotation` :type "Rotator Structure") (`Spawn Transform Scale` :type "Vector Structure") (AttachToComponent :type "SceneComponent Object Reference") (DamageTypeClass :type "DamageType Class Reference") (DamageCauser :type "Actor Object Reference") (HitInfo :type "HitResult Structure (by ref)") (HitFromDirection :type "Vector Structure (by ref)") (BaseDamage :type "Float (single-precision)") (DamagedActor :type "Actor Object Reference"))
  (`GameplayStatics.ApplyPointDamage` DamagedActor BaseDamage HitFromDirection HitInfo null DamageCauser DamageTypeClass)
  (bind _returnvalue (`|SpawnActorFromClass` "/Game/Blueprints/ClassAbilities/Ensign/EnsignFlag_BP.EnsignFlag_BP_C" (`KismetMathLibrary.MakeTransform` `Spawn Transform Location` `Spawn Transform Rotation` `Spawn Transform Scale`) "AlwaysSpawn" "MultiplyWithRoot" null null))
  (`/Game/Blueprints/ClassAbilities/Ensign/EnsignFlag_BP.SERVER_SetFlagImage` _returnvalue SteamAvatarTexture false (0.0 0.0 0.0))
  (`self.K2_AttachToComponent` _returnvalue AttachToComponent "None" "KeepWorld" "KeepWorld" "KeepWorld" true)
  (`self.K2_DestroyActor`))

(fn `UserConstructionScript`)