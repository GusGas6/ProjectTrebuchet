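; LockedOnIcon_BP is an actor that serves as a lock-on icon, keeping itself turned toward the player's camera.
; Each tick it points its X axis at the camera manager's location, resolved through the PlayerControllerREF variable, creating a billboard effect.
; It destroys itself as soon as that reference is invalid; nothing in this file sets the reference.
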(event `self.ReceiveTick`
  (params (DeltaSeconds :type "Float (single-precision)"))
  (bind _playercontrollerref (`self.PlayerControllerREF`))
  (`/Engine/EditorBlueprintResources/StandardMacros.IsValid` _playercontrollerref
    (:`Is Valid`
      (`self.K2_SetActorRotation` (`KismetMathLibrary.Conv_VectorToRotator` (`KismetMathLibrary.GetDirectionUnitVector` (`self.K2_GetActorLocation`) (`PlayerCameraManager.GetCameraLocation` (`PlayerController.PlayerCameraManager` (`PlayerState.GetPlayerController` (`Controller.PlayerState` _playercontrollerref))))))))
    (:`Is Not Valid`
      (`self.K2_DestroyActor`))))

(fn `UserConstructionScript`)