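; Test trigger that announces the boss's death and returns players to the hub level, Lvl_ThirdPerson.
; The first box overlap by a BP_ThirdPersonCharacter starts a one-time countdown, looped through a short Delay, that updates a TextRender message.
; At zero, authority and remote both fade their first player's camera and hold it.
; Only the authority then waits briefly and calls an absolute ServerTravel.
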(event `self.Box.OnComponentBeginOverlap`
  (params (OverlappedComponent :type "PrimitiveComponent Object Reference") (OtherActor :type "Actor Object Reference") (OtherComp :type "PrimitiveComponent Object Reference") (OtherBodyIndex :type Integer) (bFromSweep :type Boolean) (SweepResult :type "HitResult Structure (by ref)"))
  (bind _timeuntillaunch (`self.TimeUntilLaunch`))
  (if (== (`GameplayStatics.GetObjectClass` OtherActor) "/Game/Blueprints/BP_ThirdPersonCharacter.BP_ThirdPersonCharacter_C")
    (`/Engine/EditorBlueprintResources/StandardMacros.DoOnce` false
      (:`Completed`
        (bind _output_get (set `self.TimeUntilLaunch` (- _timeuntillaunch 0.1) :!label _label))
        (if (<= _output_get 0.0)
          (`/Engine/EditorBlueprintResources/ActorMacros.Switch Has Authority`
            (:`Authority`
              (`PlayerCameraManager.StartCameraFade` :`self` (`GameplayStatics.GetPlayerCameraManager` 0) :`ToAlpha` 1.0 :`Duration` 1.0 :`bHoldWhenFinished` true)
              (`KismetSystemLibrary.Delay` 2.0)
              (`AdvancedSessionsLibrary.ServerTravel` "Lvl_ThirdPerson" true))
            (:`Remote`
              (`PlayerCameraManager.StartCameraFade` :`self` (`GameplayStatics.GetPlayerCameraManager` 0) :`ToAlpha` 1.0 :`Duration` 1.0 :`bHoldWhenFinished` true)))
          (else
            (`TextRenderComponent.K2_SetText` (`self.TextRender`) (`KismetTextLibrary.Conv_StringToText` (`KismetStringLibrary.Concat_StrStr` "YAY BOSS IS DEAD :ddd    RETURNING TO HUB IN... " (`KismetStringLibrary.Conv_IntToString` (+ (`KismetMathLibrary.FTrunc` _timeuntillaunch) 1)))))
            (`KismetSystemLibrary.Delay` 0.1)
            (goto _label)))))))

(fn `UserConstructionScript`)